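; Trigger box actor that moves the player to the next level once the swat character meets the level's completion condition.
; On overlap it compares ItemsCount to ItemLevel0 to open Example_map_01, or to ItemLevel1, with DoorBreak also required, to open End_map.
; Both branches disable input, clear widgets, play a fade sequence and sound, then show a loading widget after a delay before opening the map.
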(event OnComponentBeginOverlap(Box)
  (params (OverlappedComponent :type Primitive%20Component%20Object%20Reference) (OtherActor :type Actor%20Object%20Reference) (OtherComp :type Primitive%20Component%20Object%20Reference) (OtherBodyIndex :type Integer) (bFromSweep :type Boolean) (SweepResult :type Hit%20Result%20Structure%20%28by%20ref%29))
  (bind _asmy_swat (Utilities|Casting|CastToMySwat OtherActor))
  (if (== (Variables|/Game/BLUEPRINT/MySwat.MySwat_C|GetItems_count _asmy_swat) (Variables|/Game/BLUEPRINT/MySwat.MySwat_C|Getitem_level0 _asmy_swat))
    (Input|DisableInput _asmy_swat 0)
    (Viewport|RemoveAllWidgets)
    (bind _returnvalue (Sequencer|Player|CreateLevelSequencePlayer "/Game/BLUEPRINT/fade_level.fade_level"))
    (Sequencer|Player|Play _returnvalue :!class /Script/MovieScene.MovieSceneSequencePlayer)
    (Audio|PlaySound2D "/Game/Sound/Zoom_Sound_Effects_All_Sounds__mp3cut_net_.Zoom_Sound_Effects_All_Sounds__mp3cut_net_")
    (Utilities|FlowControl|Delay 3.0)
    (bind _returnvalue_2 (UserInterface|CreateWidget "/Game/UI/Loading_MainMap.Loading_MainMap_C" (Game|GetPlayerController 0)))
    (UserInterface|Viewport|AddtoViewport _returnvalue_2 0)
    (Game|OpenLevel(byName) "Example_map_01")
    (elif (and (== (Variables|/Game/BLUEPRINT/MySwat.MySwat_C|GetItems_count _asmy_swat) (Variables|/Game/BLUEPRINT/MySwat.MySwat_C|Getitem_level1 _asmy_swat)) (Variables|/Game/BLUEPRINT/MySwat.MySwat_C|Getdoor_break? _asmy_swat))
      (Input|DisableInput _asmy_swat 0)
      (Viewport|RemoveAllWidgets)
      (bind _returnvalue_3 (Sequencer|Player|CreateLevelSequencePlayer "/Game/BLUEPRINT/fade_level.fade_level"))
      (Sequencer|Player|Play _returnvalue_3 :!class /Script/MovieScene.MovieSceneSequencePlayer)
      (Audio|PlaySound2D "/Game/Sound/handclap.handclap")
      (Utilities|FlowControl|Delay 3.0)
      (bind _returnvalue_4 (UserInterface|CreateWidget "/Game/UI/Loading_MainMap.Loading_MainMap_C" (Game|GetPlayerController 0)))
      (UserInterface|Viewport|AddtoViewport _returnvalue_4 0)
      (Game|OpenLevel(byName) "End_map"))))

(event EventBeginPlay)

(event Collision|EventActorBeginOverlap
  (params (OtherActor :type Actor%20Object%20Reference)))

(event EventTick
  (params (DeltaSeconds :type Float%20%28single-precision%29)))

(fn ConstructionScript)