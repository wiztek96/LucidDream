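; Magic_Plane1 is a trap-like actor that plays a sound on spawn and explodes after something overlaps it.
; Overlap swaps its mesh to a pulsing hex material, spawns a target particle and calls DestroySession, whose immediate output starts a delay before spawning the explosion and destroying itself.
; Each tick it searches all MySwat actors and adds a Timer-based local yaw for every one with IsSpin set.
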(event Collision|EventActorBeginOverlap
  (params (OtherActor :type Actor%20Object%20Reference))
  (Rendering|Material|SetMaterial (Variables|Debug|GetStaticMeshComponent) 0 "/Game/StarterContent/Materials/M_Tech_Hex_Tile_Pulse.M_Tech_Hex_Tile_Pulse")
  (Effects|SpawnEmitteratLocation "/Game/InfinityBladeEffects/Effects/FX_Monsters/FX_Monster_Ausar/P_AU_Trap_Target.P_AU_Trap_Target" (Transformation|GetWorldLocation (Variables|Default|GetBox)))
  (|DestroySession
    (:then
      (Utilities|FlowControl|Delay (Variables|Default|Gettime))
      (Game|SpawnActorfromClass "/Game/StarterContent/Blueprints/Blueprint_Effect_Explosion.Blueprint_Effect_Explosion_C" (Transformation|GetWorldTransform (Variables|Default|GetBox)) "Undefined" 0 0)
      (Actor|DestroyActor))))

(event EventTick
  (params (DeltaSeconds :type Float%20%28single-precision%29))
  (bind _outactors (Actor|GetAllActorsOfClass "/Game/BLUEPRINT/MySwat.MySwat_C"))
  (for _array_element _outactors
    (if (Variables|/Game/BLUEPRINT/MySwat.MySwat_C|GetIsSpin? _array_element)
      (Transformation|AddActorLocalRotation (Math|Rotator|MakeRotator 0.0 0.0 (+ (Variables|Default|GetTimer) 1.0)) false false))))

(event EventBeginPlay
  (Audio|PlaySoundatLocation "/Game/Sound/jump_sound_or_power_up_sound__online-audio-converter_com_.jump_sound_or_power_up_sound__online-audio-converter_com_" (Transformation|GetWorldLocation (Variables|Default|GetBox))))

(fn ConstructionScript)