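; Magic_Plane is an actor that animates its position relative to where it starts in the level.
; On BeginPlay it stores its location, then plays a timeline whose vector track is added to that origin on every update, without sweeping.
; An X-ray block that would toggle the mesh's custom depth from each MySwat's Xray flag is disconnected and never runs, leaving Tick empty.
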(event EventBeginPlay
  (Variables|Default|SetDefault_vector (Transformation|GetActorLocation))
  (bind _newtrack_2 (Timeline|Timeline_0 Play)
    (:Update
      (Transformation|SetActorLocation (+ (Variables|Default|GetDefault_vector) _newtrack_2) false false))))

(event Collision|EventActorBeginOverlap
  (params (OtherActor :type Actor%20Object%20Reference)))

(event EventTick
  (params (DeltaSeconds :type Float%20%28single-precision%29))
  ;[1 1 1] Active Xray from MySwat
)

(fn ConstructionScript)