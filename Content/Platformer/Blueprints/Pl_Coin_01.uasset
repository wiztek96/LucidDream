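; Collectible coin for the platformer that spins every tick and is picked up when the MySwat player overlaps it.
; Pickup increments the player's item count, updates and scales the HUD counter, plays particles and sound, then destroys the coin.
; Reaching the level's item target triggers the HUD's level-complete call.
; While the cached MySwat's Xray flag is on, the mesh renders to custom depth.
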(event Collision|EventActorBeginOverlap
  (params (OtherActor :type Actor%20Object%20Reference))
  (bind _asmy_swat (Utilities|Casting|CastToMySwat OtherActor))
  (Default|ScaleItem (Variables|/Game/BLUEPRINT/MySwat.MySwat_C|GetHUD_ref _asmy_swat))
  (bind _output_get (Variables|/Game/BLUEPRINT/MySwat.MySwat_C|SetItems_count _asmy_swat (+ (Variables|/Game/BLUEPRINT/MySwat.MySwat_C|GetItems_count _asmy_swat) 1)))
  (bind _foundwidgets (Widget|GetAllWidgetsOfClass "/Game/UI/MainHUD/HUD_main.HUD_main_C" true))
  (for _array_element _foundwidgets
    (Rendering|Components|TextRender|SetText (Variables|/Game/UI/MainHUD/HUD_main.HUD_main_C|GetItem_count _array_element) (Utilities|Text|ToText(Integer) _output_get))
    (Effects|SpawnEmitteratLocation "/Game/InfinityBladeEffects/Effects/FX_Combat_Base/WeaponCombo/P_ComboFinish_Tap_01.P_ComboFinish_Tap_01" (Transformation|GetWorldLocation (Variables|Default|GetStaticMesh)) "0, 0, 0" false)
    (Audio|PlaySoundatLocation "/Game/Sound/Super_Mario_Bros_-Coin_Sound_Effect-RfkcI8dhfsQ.Super_Mario_Bros_-Coin_Sound_Effect-RfkcI8dhfsQ" "0, 0, 0")
    (Actor|DestroyActor)
    (Variables|Default|SetDestroyed? true)
    (if (== (Variables|/Game/BLUEPRINT/MySwat.MySwat_C|GetItems_count _asmy_swat) (Variables|/Game/BLUEPRINT/MySwat.MySwat_C|Getitem_level1 _asmy_swat))
      (Default|ItemLevelComplete (Variables|/Game/BLUEPRINT/MySwat.MySwat_C|GetHUD_ref _asmy_swat)))))

(event EventTick
  (params (DeltaSeconds :type Float%20%28single-precision%29))
  (bind _staticmesh (Variables|Default|GetStaticMesh))
  (Transformation|AddActorLocalRotation "0,5.000000, 0" false false)
  (if (not (Variables|Default|GetDestroyed?))
    (if (Variables|/Game/BLUEPRINT/MySwat.MySwat_C|GetXray? (stale EventBeginPlay _array_element))
      (Rendering|SetRenderCustomDepth _staticmesh true)
      (else
        (Rendering|SetRenderCustomDepth _staticmesh false)))))

(event EventBeginPlay
  (bind _outactors (Actor|GetAllActorsOfClass "/Game/BLUEPRINT/MySwat.MySwat_C"))
  (for _array_element _outactors
    _))

(fn ConstructionScript)