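; Collectible item pickup for a platformer that spins in place and counts toward completing the level.
; A timeline update rotates it and polls every MySwat's Xray flag to toggle custom depth on its mesh.
; On MySwat overlap it increments the player's item count, updates the HUD, plays effects and destroys itself.
; When the count reaches ItemLevel0, it spawns portal particles at Box_levelup actors and signals item completion on the HUD.
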(event Collision|EventActorBeginOverlap
  (params (OtherActor :type Actor%20Object%20Reference))
  (bind _asmy_swat (Utilities|Casting|CastToMySwat OtherActor))
  (Default|ScaleItem (Variables|/Game/BLUEPRINT/MySwat.MySwat_C|GetHUD_ref _asmy_swat))
  (bind _output_get (Variables|/Game/BLUEPRINT/MySwat.MySwat_C|SetItems_count _asmy_swat (+ (Variables|/Game/BLUEPRINT/MySwat.MySwat_C|GetItems_count _asmy_swat) 1)))
  (bind _foundwidgets (Widget|GetAllWidgetsOfClass "/Game/UI/MainHUD/HUD_main.HUD_main_C" true))
  (for _array_element _foundwidgets
    (Rendering|Components|TextRender|SetText (Variables|/Game/UI/MainHUD/HUD_main.HUD_main_C|GetItem_count _array_element) (Utilities|Text|ToText(Integer) _output_get))
    (Effects|SpawnEmitteratLocation "/Game/InfinityBladeEffects/Effects/FX_Mobile/Fire/combat/P_MovingSpin_Fire_Charge_01.P_MovingSpin_Fire_Charge_01" (Transformation|GetWorldLocation (Variables|Default|GetStaticMesh)))
    (Audio|PlaySoundatLocation "/Game/Sound/power_up_grab__online-audio-converter_com_.power_up_grab__online-audio-converter_com_" "0, 0, 0")
    (Actor|DestroyActor)
    (Variables|Default|SetDestroyed? true)
    (if (== (Variables|/Game/BLUEPRINT/MySwat.MySwat_C|GetItems_count _asmy_swat) (Variables|/Game/BLUEPRINT/MySwat.MySwat_C|Getitem_level0 _asmy_swat))
      (bind _outactors (Actor|GetAllActorsOfClass "/Game/BLUEPRINT/box_levelup.box_levelup_C"))
      (for _array_element_2 _outactors
        (Effects|SpawnEmitteratLocation "/Game/AURA/Aura_portal_particles.Aura_portal_particles" (Transformation|GetActorLocation _array_element_2))
        (Default|ItemLevelComplete _array_element)))))

(event EventBeginPlay
  (bind _staticmesh (Variables|Default|GetStaticMesh))
  (Timeline|Timeline_0 Play
    (:Update
      (Transformation|AddActorLocalRotation "0,5.000000, 0" false false)
      ;[1 1 1] Active Xray from MySwat
      (if (not (Variables|Default|GetDestroyed?))
        (bind _outactors (Actor|GetAllActorsOfClass "/Game/BLUEPRINT/MySwat.MySwat_C"))
        (for _array_element _outactors
          (if (Variables|/Game/BLUEPRINT/MySwat.MySwat_C|GetXray? _array_element)
            (Rendering|SetRenderCustomDepth _staticmesh true)
            (else
              (Rendering|SetRenderCustomDepth _staticmesh false))))))))

(fn ConstructionScript)