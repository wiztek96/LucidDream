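; SkyBox_BP is a sky sphere actor that blacks out the sky when a MySwat character has Xray active.
; The construction script applies SkyMaterial to the sphere.
; Every Tick it searches for all MySwat actors and sets the black skybox material or SkyMaterial from each one's Xray flag, so the last actor in the list decides the result.
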(event EventBeginPlay)

(event EventTick
  (params (DeltaSeconds :type Float%20%28single-precision%29))
  (bind _outactors (Actor|GetAllActorsOfClass "/Game/BLUEPRINT/MySwat.MySwat_C"))
  (for _array_element _outactors
    (if (Variables|/Game/BLUEPRINT/MySwat.MySwat_C|GetXray? _array_element)
      (Rendering|Material|SetMaterial (Variables|Default|GetSkyshpere) 0 "/Game/StarterContent/Blueprints/Assets/M_LightStage_Skybox_Black.M_LightStage_Skybox_Black")
      (else
        (Rendering|Material|SetMaterial (Variables|Default|GetSkyshpere) 0 (Variables|Default|GetSky_material))))))

(fn ConstructionScript
  (Rendering|Material|SetMaterial (Variables|Default|GetSkyshpere) 0 (Variables|Default|GetSky_material)))